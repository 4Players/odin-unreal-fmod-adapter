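; Player controller that connects the local player to an ODIN voice chat room, with remote voices played back through FMOD adapters.
; On BeginPlay it generates a token client-side, constructs a room with audio-processing settings and joins.
; On success it streams captured audio and has the controlled character replicate its peer ID.
; Media events update a peer-to-media map and create or destroy adapters on characters found by peer ID.
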(event `self.ReceiveBeginPlay`
  ;[1 1 1] Ensure we only join the odin room once.
  (if (`self.IsLocalPlayerController`)
    (`self.Join Odin Room`)))

(event `Join Odin Room`
  ;[1 1 1] Run on client only and once only
  (`|ExecutionSequence`
    (:`then_0`
      ;[1 1 1] Setup Odin
      ;;[1 1 1] Generate Room Token. Please Note: In production environments we recommend doing this only on a secured server to avoid leaking your access key to the public. See: https://www.4players.io/odin/introduction/access-keys/
      (bind _returnvalue (`OdinTokenGenerator.GenerateRoomToken` (`OdinTokenGenerator.ConstructTokenGenerator` (`self.Access Key`)) (`self.Room Name`) "My User Id" "Default"))
      (set `self.RoomToken` _returnvalue)
      ;;[1 1 1] Construct Room Handle with applied settings
      (set `self.RoomHandle` (`OdinRoom.ConstructRoom` (make `OdinApmSettings` true 0.6 0.5 true -40.0 -30.0 true true true "OdinNS_Moderate" true))))
    (:`then_1`
      ;[1 1 1] On Media Added
      (add `OdinRoom.onMediaAdded` (`self.RoomHandle`) (delegate `OnMediaAdded`)))
    (:`then_2`
      ;[1 1 1] On Media Removed
      (add `OdinRoom.onMediaRemoved` (`self.RoomHandle`) (delegate `OnMediaRemoved`)))
    (:`then_3`
      ;[1 1 1] Join Odin Room
      (`OdinRoomJoin.JoinRoom` :`room` (`self.RoomHandle`) :`url` (`self.ServerUrl`) :`token` (`self.RoomToken`) :`onSuccess` (delegate `OnJoinRoomSuccess`)))))

(event `OnMediaAdded`
  (params (peerId :type Integer64) (media :type "OdinPlaybackMedia Object Reference") (properties :type "OdinJsonObject Object Reference") (room :type "OdinRoom Object Reference"))
  (bind (_value _returnvalue) (`BlueprintMapLibrary.Map_Find` (`self.PeerToChar`) peerId))
  ;[1 1 1] On Media Added
  (`BlueprintMapLibrary.Map_Add` (`self.PeerToMedia`) peerId media)
  ;;[1 1 1] If the peer id has been replicated before the media added event, create odin synth on registered remote character
  (if _returnvalue
    (`/OdinFmodAdapter/Blueprints/BP_OdinFmodMultiplayerCharacter.CreateOdinFmodAdapter` _value media)))

(event `OnMediaRemoved`
  (params (peerId :type Integer64) (media :type "OdinPlaybackMedia Object Reference") (room :type "OdinRoom Object Reference"))
  (bind (_value _returnvalue) (`BlueprintMapLibrary.Map_Find` (`self.PeerToChar`) peerId))
  (bind _returnvalue_2 (`self.GetComponentByClass` _value "/Script/OdinFmodAdapter.OdinFmodAdapterComponent"))
  ;[1 1 1] On Media Removed
  ;;[1 1 1] Destroy Odin Synth Component which has been playing back audio from the removed media
  (`BlueprintMapLibrary.Map_Remove` (`self.PeerToMedia`) peerId)
  (if _returnvalue
    (`/Engine/EditorBlueprintResources/StandardMacros.IsValid` _returnvalue_2
      (:`Is Valid`
        (`ActorComponent.K2_DestroyComponent` _returnvalue_2)))))

(event `OnJoinRoomSuccess`
  (params (roomId :type String) (roomUserData :type "Array of Byte (by ref)") (customer :type String) (ownPeerId :type Integer64) (ownUserId :type String))
  ;[1 1 1] Join Odin Room
  ;;[1 1 1] Setup Audio Capture and connect to Odin Room
  (bind _returnvalue (`OdinFunctionLibrary.CreateOdinAudioCapture`))
  (`AudioCapture.StartCapturingAudio` _returnvalue)
  (`OdinRoomAddMedia.AddMedia` (`self.RoomHandle`) (`OdinFunctionLibrary.Odin_CreateMedia` _returnvalue)
    (:`then`
      ;;[1 1 1] Replicate characters peer id to remote clients
      (bind _asbp_odin_fmod_multiplayer_character (cast `/OdinFmodAdapter/Blueprints/BP_OdinFmodMultiplayerCharacter` (`self.K2_GetPawn`)))
      (`/OdinFmodAdapter/Blueprints/BP_OdinFmodMultiplayerCharacter.ReplicatePeerId` _asbp_odin_fmod_multiplayer_character ownPeerId))))

(fn `UserConstructionScript`)